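; Weather controller that switches the scene between weather types, driving particles, material parameters and sky lighting.
; Activation puts the current type's particle template on the player character and plays a timeline that ramps its Material Parameter Collection scalar while zeroing the previous type's.
; Each timeline update also interpolates sky sphere values and directional light color toward the current type's settings.
; Transitions deactivate, reversing the timeline, then activate after a short delay.
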(event `self.ActivateCurrentWeatherEffect`
  (bind _currentweathertype (`self.CurrentWeatherType`))
  (bind _currentweathertype_2 (`self.CurrentWeatherType`))
  (bind _particlesystem (`/Game/ThirdPersonCPP/Blueprints/ThirdPersonCharacter.ParticleSystem` (cast `/Game/ThirdPersonCPP/Blueprints/ThirdPersonCharacter` (`GameplayStatics.GetPlayerCharacter` 0) :!pure true)))
  (bind _weatherparticlesystem (`WeatherType.WeatherParticleSystem` (`self.CurrentWeatherType`))
    (:`then`
      (`ParticleSystemComponent.SetTemplate` _particlesystem _weatherparticlesystem)
      (`ActorComponent.Activate` _particlesystem false)
      (set `self.Weather Particle System` _particlesystem))
    (:`else`
      _))
  (`WeatherType.MaterialParamCollection` _currentweathertype
    (:`then`
      (`TimelineComponent.SetPlayRate` (`self.MPC Timeline`) (/ 1.0 (`WeatherType.MPC_TransitionTime` _currentweathertype)))
      (`KismetMaterialLibrary.SetScalarParameterValue` (`WeatherType.MaterialParamCollection` _currentweathertype) (`WeatherType.MPC_ParamName` _currentweathertype))
      (bind (_direction _reversable_float_track) (`Timeline|MPC Timeline` :!label _label)
        (:`Update`
          (bind _materialparamcollection (`WeatherType.MaterialParamCollection` _currentweathertype_2)
            (:`then`
              (`KismetMaterialLibrary.SetScalarParameterValue` _materialparamcollection (`WeatherType.MPC_ParamName` _currentweathertype_2) (* _reversable_float_track 0.1)))
            (:`else`
              _))
          (bind _previous_weather_type (`self.Previous Weather Type`)
            (:`then`
              (bind _materialparamcollection_2 (`WeatherType.MaterialParamCollection` _previous_weather_type)
                (:`then`
                  (`KismetMaterialLibrary.SetScalarParameterValue` _materialparamcollection_2 (`WeatherType.MPC_ParamName` _previous_weather_type)))
                (:`else`
                  _)))
            (:`else`
              _))
          (`self.Sky Sphere Reference`
            (:`then`
              (`self.SetSkySphereValues`))
            (:`else`)))
        (:`Finished`
          (set `self.Previous Weather Type` _currentweathertype_2))))
    (:`else`
      (goto _label))))

(event `self.DeactivateCurrentWeatherEffect`
  (`ActorComponent.Deactivate` (`self.Weather Particle System`))
  (goto _label :!via `Reverse`))

(event `self.TransitionBetweenWeatherEffects`
  (`self.DeactivateCurrentWeatherEffect`)
  (`KismetSystemLibrary.Delay` 1.0)
  (`self.ActivateCurrentWeatherEffect`))

(fn `SetSkySphereValues`
  (bind _sky_sphere_reference (`self.Sky Sphere Reference`))
  (bind _transitionspeed (`self.TransitionSpeed`))
  (bind _sky_sphere_reference_2 (`self.Sky Sphere Reference`))
  (bind _transitionspeed_2 (`self.TransitionSpeed`))
  (bind _sky_sphere_reference_3 (`self.Sky Sphere Reference`))
  (bind _transitionspeed_3 (`self.TransitionSpeed`))
  (bind _currentweathertype (`self.CurrentWeatherType`))
  (bind _currentweathertype_2 (`self.CurrentWeatherType`))
  (bind _currentweathertype_3 (`self.CurrentWeatherType`))
  (bind _currentweathertype_4 (`self.CurrentWeatherType`))
  (bind _transitionspeed_4 (`self.TransitionSpeed`))
  (bind _sky_sphere_reference_4 (`self.Sky Sphere Reference`))
  (bind _directional_light_actor (`/Engine/EngineSky/BP_Sky_Sphere.Directional light actor` _sky_sphere_reference)
    (:`then`
      (bind _lightcomponent (`Light.LightComponent` _directional_light_actor))
      (`LightComponent.SetLightColor` _lightcomponent (`KismetMathLibrary.CInterpTo` (`LightComponentBase.GetLightColor` _lightcomponent) (`WeatherType.SceneLightingColor` _currentweathertype) 1.0 _transitionspeed_4) true)
      (set `/Engine/EngineSky/BP_Sky_Sphere.Horizon Falloff` (`KismetMathLibrary.FInterpTo` (`/Engine/EngineSky/BP_Sky_Sphere.Horizon Falloff` _sky_sphere_reference) (`WeatherType.HorizonFalloff` _currentweathertype) 1.0 _transitionspeed_4) _sky_sphere_reference)
      (set `/Engine/EngineSky/BP_Sky_Sphere.Sun brightness` (`KismetMathLibrary.FInterpTo` (`/Engine/EngineSky/BP_Sky_Sphere.Sun brightness` _sky_sphere_reference_4) (`WeatherType.SunBrightness` _currentweathertype_2) 1.0 _transitionspeed) _sky_sphere_reference_4)
      (set `/Engine/EngineSky/BP_Sky_Sphere.Cloud speed` (`KismetMathLibrary.FInterpTo` (`/Engine/EngineSky/BP_Sky_Sphere.Cloud speed` _sky_sphere_reference_4) (`WeatherType.CloudSpeed` _currentweathertype_2) 1.0 _transitionspeed) _sky_sphere_reference_4)
      (set `/Engine/EngineSky/BP_Sky_Sphere.Cloud opacity` (`KismetMathLibrary.FInterpTo` (`/Engine/EngineSky/BP_Sky_Sphere.Cloud opacity` _sky_sphere_reference_2) (`WeatherType.CloudOpacity` _currentweathertype_3) 1.0 _transitionspeed_2) _sky_sphere_reference_2)
      (set `/Engine/EngineSky/BP_Sky_Sphere.Zenith Color` (`KismetMathLibrary.CInterpTo` (`/Engine/EngineSky/BP_Sky_Sphere.Zenith Color` _sky_sphere_reference_2) (`WeatherType.ZenithColor` _currentweathertype_3) 1.0 _transitionspeed_2) _sky_sphere_reference_2)
      (set `/Engine/EngineSky/BP_Sky_Sphere.Horizon color` (`KismetMathLibrary.CInterpTo` (`/Engine/EngineSky/BP_Sky_Sphere.Horizon color` _sky_sphere_reference_3) (`WeatherType.HorizonColor` _currentweathertype_4) 1.0 _transitionspeed_3) _sky_sphere_reference_3)
      (set `/Engine/EngineSky/BP_Sky_Sphere.Cloud color` (`KismetMathLibrary.CInterpTo` (`/Engine/EngineSky/BP_Sky_Sphere.Cloud color` _sky_sphere_reference_3) (`WeatherType.CloudColor` _currentweathertype_4) 1.0 _transitionspeed_3) _sky_sphere_reference_3)
      (set `/Engine/EngineSky/BP_Sky_Sphere.Overall Color` (`KismetMathLibrary.CInterpTo` (`/Engine/EngineSky/BP_Sky_Sphere.Overall Color` _sky_sphere_reference_3) (`WeatherType.OverallSkyColor` _currentweathertype_4) 1.0 _transitionspeed_3) _sky_sphere_reference_3)
      (`/Engine/EngineSky/BP_Sky_Sphere.RefreshMaterial` _sky_sphere_reference_3))
    (:`else`)))

(fn `UserConstructionScript`)